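; Survival game mode that presents wave progress and the win or lose ending, with boss battle music started at BeginPlay.
; It binds to the survival state-change delegate and switches on each state to show wave banners, with or without countdowns.
; The last wave also sets the enemy spawn delay and gets an extra banner.
; Victory or player death clears widgets, fades out the camera, then async-loads the matching end screen.
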(event Custom|OnSurvivalGameModeStateChanged_이벤트
  (params (CurrentState :type EWarriorSurvivalGameModeState%20Enum :default "WaitSpawnNewWave"))
  (switch Utilities|FlowControl|Switch|SwitchonEWarriorSurvivalGameModeState CurrentState
    (:WaitSpawnNewWave
      (CallFunction|CreateWaveWidgetwithCountDown "New WAve Coming In" (Variables|Default|GetSpawnNewWaveWaitTime)))
    (:SpawningNewWave
      (CallFunction|CreateWaveWidgetNoCountDown (Utilities|Text|FormatText "Wave {CurrentWaveCount}" (Variables|Default|GetCurrentWaveCount)))
      (if (== (Variables|Default|GetTotalWavesToSpawn) (Variables|Default|GetCurrentWaveCount))
        (Variables|Default|SetSpawnEnemiesDelayTime 4.0)
        (Utilities|FlowControl|Delay 2.0)
        (CallFunction|CreateWaveWidgetNoCountDown "LAst Wave")))
    (:WaveCompleted
      (CallFunction|CreateWaveWidgetwithCountDown (Utilities|Text|FormatText "Wave {CurrentWaveCount} Completed" (Variables|Default|GetCurrentWaveCount)) (Variables|Default|GetWaveCompletedWaitTime)))
    (:AllWavesDone
      (Utilities|FlowControl|Delay 1.5)
      (Viewport|RemoveAllWidgets)
      (CameraFades|StartCameraFade :self (Game|GetPlayerCameraManager 0) :ToAlpha 1.0 :Duration 3.0 :bHoldWhenFinished true)
      (Utilities|FlowControl|Delay 3.0)
      (bind _class (Utilities|AsyncLoadClassAsset "/Game/Widgets/GameModeWidgets/WBP_WinScreen.WBP_WinScreen_C")
        (:Completed
          (bind _as사용자_위젯 (Utilities|Casting|CastToUserWidgetClass _class))
          (bind _returnvalue (UserInterface|CreateWidget _as사용자_위젯))
          (UserInterface|Viewport|AddtoViewport _returnvalue 0))))
    (:PlayerDied
      (Viewport|RemoveAllWidgets)
      (CameraFades|StartCameraFade :self (Game|GetPlayerCameraManager 0) :ToAlpha 1.0 :Duration 2.0 :bHoldWhenFinished true)
      (Utilities|FlowControl|Delay 2.0)
      (bind _class_2 (Utilities|AsyncLoadClassAsset "/Game/Widgets/GameModeWidgets/WBP_LoseScreen.WBP_LoseScreen_C")
        (:Completed
          (bind _as사용자_위젯_2 (Utilities|Casting|CastToUserWidgetClass _class_2))
          (bind _returnvalue_2 (UserInterface|CreateWidget _as사용자_위젯_2))
          (UserInterface|Viewport|AddtoViewport _returnvalue_2 0))))))

(event EventBeginPlay
  (Audio|SpawnSound2D "/Game/Assets/Sounds/Music/Dungeons_EndBossBattle.Dungeons_EndBossBattle" 1.0 1.0 0.0 0)
  (EventDispatchers|AssignOnSurvivalGameModeStateChanged (delegate Custom|OnSurvivalGameModeStateChanged_이벤트)))

(event EventTick
  (params (DeltaSeconds :type Float%20%28single-precision%29)))

(fn ConstructionScript)

(fn CreateWaveWidgetwithCountDown
  (params (TextContentToDisplay :type Text) (InTotalCountDownTime :type Float%20%28double-precision%29))
  (bind _returnvalue (UserInterface|CreateWidget "/Game/Widgets/GameModeWidgets/WBP_WaveTextWWithCountDown.WBP_WaveTextWWithCountDown_C"))
  (UserInterface|Viewport|AddtoViewport _returnvalue 0)
  (Rendering|Components|TextRender|SetText (Variables|/Game/Widgets/GameModeWidgets/WBP_WaveTextWWithCountDown.WBP_WaveTextWWithCountDown_C|GetTextBlock_WaveText _returnvalue) TextContentToDisplay)
  (Default|StartCountDown _returnvalue InTotalCountDownTime))

(fn CreateWaveWidgetNoCountDown
  (params (TextContentToDisplay :type Text))
  (bind _returnvalue (UserInterface|CreateWidget "/Game/Widgets/GameModeWidgets/WBP_WaveTextWNoCountDown.WBP_WaveTextWNoCountDown_C"))
  (UserInterface|Viewport|AddtoViewport _returnvalue 0)
  (Rendering|Components|TextRender|SetText (Variables|/Game/Widgets/GameModeWidgets/WBP_WaveTextWNoCountDown.WBP_WaveTextWNoCountDown_C|GetTextBlock_WaveText _returnvalue) TextContentToDisplay))